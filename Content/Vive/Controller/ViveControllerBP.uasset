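; Vive motion-controller hand that lets the player climb and grasp objects in VR.
; A per-tick sphere check at the grab point and mesh overlaps flag Climbable actors, so GrabActor either calls the owner's ClimbingComponent or grasps the nearest GraspableActor's closest region.
; ReleaseActor ends climbing and drops the gripped region, adjusting hand collision profiles, with a delay before restoring Hand.
; Bone hits rumble the matching side, scaled by controller velocity.
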(event OnComponentBeginOverlap(ControllerMesh)
  (params (OverlappedComponent :type Primitive%20Component%20Object%20Reference) (OtherActor :type Actor%20Object%20Reference) (OtherComp :type Primitive%20Component%20Object%20Reference) (OtherBodyIndex :type Integer) (bFromSweep :type Boolean) (SweepResult :type Hit%20Result%20Structure%20%28by%20ref%29))
  (if (Actor|ActorHasTag OtherActor (Variables|Default|GetClimbable))
    (if (== (Variables|Default|GetAttachedActor) 0)
      (Variables|Default|SetbWantsToClimb true))))

(event OnComponentEndOverlap(ControllerMesh)
  (params (OverlappedComponent :type Primitive%20Component%20Object%20Reference) (OtherActor :type Actor%20Object%20Reference) (OtherComp :type Primitive%20Component%20Object%20Reference) (OtherBodyIndex :type Integer))
  (Variables|Default|SetbWantsToClimb false))

(event OnComponentHit(Bones)
  (params (HitComponent :type Primitive%20Component%20Object%20Reference) (OtherActor :type Actor%20Object%20Reference) (OtherComp :type Primitive%20Component%20Object%20Reference) (NormalImpulse :type Vector :default "0, 0, 0") (Hit :type Hit%20Result%20Structure%20%28by%20ref%29))
  (bind _hand (Variables|Default|GetHand))
  (bind _returnvalue (Utilities|Select :Index _hand :Left true :Right false :AnyHand false :Pad false :ExternalCamera false :Gun false :Special_1 false :Special_2 false :Special_3 false :Special_4 false :Special_5 false :Special_6 false :Special_7 false :Special_8 false :Special_9 false :Special_10 false :Special_11 false))
  (bind _returnvalue_2 (not _returnvalue))
  ;[1 1 1] Rumble When Colliding
  (Utilities|FlowControl|Sequence
    (:then_0
      (bind _returnvalue_3 (Physics|GetPhysicsLinearVelocity (Variables|Default|GetControllerMesh) "None"))
      (Game|Feedback|PlayDynamicForceFeedback (Game|GetPlayerController 0) (* (Math|Vector|VectorLength _returnvalue_3) (Variables|Default|GetForceScale)) 0.04 _returnvalue _returnvalue _returnvalue_2 _returnvalue_2))))

(event Custom|DelayedDrop
  (params (Region :type Graspable%20Region%20Object%20Reference))
  (Utilities|IsValid (Class|GraspableRegion|GetGraspedComponent Region)
    (:Is%20Valid
      (Collision|SetCollisionProfileName (Variables|Default|GetBones) "OverlapAllHand" :!class /Script/Engine.PrimitiveComponent))
    (:Is%20Not%20Valid
      (Class|GraspableRegion|Release Region (Variables|Default|GetParent))
      (Utilities|FlowControl|Delay 0.2)
      (Collision|SetCollisionProfileName (Variables|Default|GetBones) "Hand" :!class /Script/Engine.PrimitiveComponent))))

(event EventBeginPlay
  (Collision|SetCollisionEnabled (Variables|Default|GetBones) "QueryAndPhysics"))

(event Collision|EventActorBeginOverlap
  (params (OtherActor :type Actor%20Object%20Reference)))

(event EventTick
  (params (DeltaSeconds :type Float%20%28single-precision%29))
  (Utilities|FlowControl|Sequence
    (:then_0
      (Variables|Default|SetbWantsToClimb false)
      (bind _outactors (Collision|SphereOverlapActors (Transformation|GetWorldLocation (Variables|Default|GetGrab%20Point)) 0.1 (Utilities|Array|MakeArray "ObjectTypeQuery1") "/Script/Engine.Actor"))
      (bind _array_element (Utilities|Array|ForEachLoopwithBreak _outactors :!label _label)
        (:LoopBody
          (if (Actor|ActorHasTag _array_element (Variables|Default|GetClimbable))
            (Variables|Default|SetbWantsToClimb true)
            (goto _label Break)))))))

(fn ConstructionScript
  (Variables|Default|SetHand (Variables|Default|GetHand)))

(fn GetActorNearHand
  (bind _grab_point (Variables|Default|GetGrab%20Point))
  (for _array_element (Collision|GetOverlappingActors _grab_point "/Script/MyProject3.GraspableActor" :!class /Script/Engine.PrimitiveComponent)
    (if (< (Math|Vector|VectorLength (- (Transformation|GetActorLocation _array_element) (Transformation|GetWorldLocation _grab_point))) (LocalVariables|GetNearestOverlap))
      (LocalVariables|SetNearestOverlappingActor _array_element)
      (LocalVariables|SetNearestOverlap (Math|Vector|VectorLength (- (Transformation|GetActorLocation _array_element) (Transformation|GetWorldLocation _grab_point))))))
  (return (LocalVariables|GetNearestOverlappingActor)))

(fn ReleaseActor
  (bind _grippedregion (Variables|Default|GetGrippedRegion))
  (bind _grippedregion_2 (Variables|Default|GetGrippedRegion))
  (Default|ReleaseClimbable (Variables|/Game/Vive/VRPawn.VRPawn_C|GetClimbingComponent (Variables|Default|GetOwnerActor)))
  (Variables|Default|SetbWantsToGrip false)
  (Utilities|IsValid (Variables|Default|GetAttachedActor)
    (:Is%20Valid
      (Utilities|IsValid _grippedregion
        (:Is%20Valid
          (CallFunction|DelayedDrop _grippedregion))))
    (:Is%20Not%20Valid
      (Utilities|IsValid _grippedregion_2
        (:Is%20Valid
          (CallFunction|DelayedDrop _grippedregion_2))
        (:Is%20Not%20Valid
          _))))
  (Variables|Default|SetAttachedActor 0) ; Clear the reference
)

(fn GrabActor
  (if (Variables|Default|GetbWantsToClimb)
    (Default|GrabClimbable (Variables|/Game/Vive/VRPawn.VRPawn_C|GetClimbingComponent (Variables|Default|GetOwnerActor)))
    (else
      ;[1 1 1] Simple Grab
      (bind _nearestmesh (CallFunction|GetActorNearHand))
      (Utilities|IsValid _nearestmesh
        (:Is%20Valid
          (bind _output_get (Variables|Default|SetAttachedActor _nearestmesh))
          (bind _asgraspable_actor (Utilities|Casting|CastToGraspableActor _output_get))
          (bind (_outhint _returnvalue) (Class|GraspableInterface|FindGraspableRegionNearestto(Message) _asgraspable_actor (Utilities|Struct|MakeHandInformation "Hand" (Transformation|GetWorldTransform (Variables|Default|GetGrab%20Point))) 3e+01))
          (Rendering|Components|TextRender|SetText (Variables|Default|GetInfo) (Utilities|Text|ToText(String) (Utilities|GetObjectName _returnvalue)))
          (CallFunction|GrabRegion _returnvalue _outhint))))))

(fn GrabRegion
  (params (RegionToGrasp :type Graspable%20Region%20Object%20Reference) (GraspableRegionHint :type Grip%20Hint%20Structure))
  (Variables|Default|SetGraspableRegionHint GraspableRegionHint)
  (bind _output_get (Variables|Default|SetGrippedRegion RegionToGrasp))
  (Utilities|IsValid _output_get
    (:Is%20Valid
      (bind _output_get_2 (LocalVariables|SetGraspedComponent (Class|GraspableRegion|GetGraspedComponent RegionToGrasp)))
      (Utilities|IsValid _output_get_2
        (:Is%20Valid
          (Utilities|FlowControl|Sequence
            (:then_0
              (LocalVariables|SetCanBeGrasped (.CanBeGrasped (Utilities|Struct|BreakGripHint (Variables|Default|GetGraspableRegionHint)))))
            (:then_1
              (LocalVariables|SetTransformIsRelative (.RelativeTransform (Utilities|Struct|BreakGripHint (Variables|Default|GetGraspableRegionHint)))))
            (:then_2
              (LocalVariables|SetTransform (.Transform (Utilities|Struct|BreakGripHint (Variables|Default|GetGraspableRegionHint)))))
            (:then_3
              (if (LocalVariables|GetCanBeGrasped)
                (Class|GraspableRegion|Grasp (Variables|Default|GetGrippedRegion) (Variables|Default|GetParent) "ECC_GameTraceChannel2")
                (if (LocalVariables|GetTransformIsRelative)
                  (Variables|Default|SetOffset (Utilities|GetHandOffset))
                  (else
                    (Variables|Default|SetOffset "")))))))
        (:Is%20Not%20Valid
          ;[1 1 1] Grasp this region in case its an activator.
          (Class|GraspableRegion|Grasp (Variables|Default|GetGrippedRegion) (Variables|Default|GetParent) "ECC_GameTraceChannel2"))))))